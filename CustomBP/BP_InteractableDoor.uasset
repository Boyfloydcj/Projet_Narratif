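; BP_InteractableDoor is a door that toggles open and closed on Interact and can require an inventory item.
; IsPlayerCharacterInteractable selects whether the first-person character or other actors trigger it.
; A sufficient item count unlocks it, optionally consuming the items, leaving the swing to the next interaction.
; A FlipFlop plays or reverses a yaw timeline and swaps the look-at action name, also firing at BeginPlay for doors starting open.
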(event EventInteract
  (params (ActorTriggeringInereact :type Actor%20Object%20Reference))
  (bind _isplayercharacterinteractable (Variables|Default|GetIsPlayerCharacterInteractable))
  (bind _itemid (Variables|Default|GetItemID))
  (bind _asbp_first_person_character (Utilities|Casting|CastToBP_FirstPersonCharacter ActorTriggeringInereact)
    (:then
      (if _isplayercharacterinteractable
        (if (Variables|Default|GetIsItemNeeded) :!label _label
          (if (.ReturnValue (Utilities|Map|Find (Variables|/Game/FirstPerson/Blueprints/BP_FirstPersonCharacter.BP_FirstPersonCharacter_C|GetInventory _asbp_first_person_character) (Variables|Default|GetItemID)))
            (if (>= (.Value (Utilities|Map|Find (Variables|/Game/FirstPerson/Blueprints/BP_FirstPersonCharacter.BP_FirstPersonCharacter_C|GetInventory _asbp_first_person_character) (Variables|Default|GetItemID))) (Variables|Default|GetAmountOfItemNeeded))
              (Variables|Default|SetIsItemNeeded false)
              (if (Variables|Default|GetIsItemRemoved)
                (Utilities|Map|Add (Variables|/Game/FirstPerson/Blueprints/BP_FirstPersonCharacter.BP_FirstPersonCharacter_C|GetInventory _asbp_first_person_character) _itemid (- (.Value (Utilities|Map|Find (Variables|/Game/FirstPerson/Blueprints/BP_FirstPersonCharacter.BP_FirstPersonCharacter_C|GetInventory _asbp_first_person_character) _itemid)) (Variables|Default|GetAmountOfItemNeeded))))
              (if (stale _isa)
                (Variables|Default|SetLook_at_action_name (Variables|Default|GetActionNameForA))
                (else
                  (Variables|Default|SetLook_at_action_name (Variables|Default|GetActionNameForB))))))
          (else
            (bind _isa (Utilities|FlowControl|FlipFlop)
              (:A
                (Variables|Default|SetLook_at_action_name (Variables|Default|GetActionNameForA))
                (bind _newangleovertime (Timeline|TL_MoveDoor Play)
                  (:Update
                    (Transformation|SetRelativeRotation (Variables|Default|GetDoor) (Math|Rotator|MakeRotator 0.0 0.0 _newangleovertime) false false))))
              (:B
                (Variables|Default|SetLook_at_action_name (Variables|Default|GetActionNameForB))
                (Timeline|TL_MoveDoor Reverse)))))))
    (:CastFailed
      (if (not _isplayercharacterinteractable)
        (goto _label)))))

(event EventBeginPlay
  (if (Variables|Default|GetIsOpenAtStart)
    (bind _isa (Utilities|FlowControl|FlipFlop)
      (:A
        (Variables|Default|SetLook_at_action_name (Variables|Default|GetActionNameForA))
        (bind _newangleovertime (Timeline|TL_MoveDoor Play)
          (:Update
            (Transformation|SetRelativeRotation (Variables|Default|GetDoor) (Math|Rotator|MakeRotator 0.0 0.0 _newangleovertime) false false))))
      (:B
        (Variables|Default|SetLook_at_action_name (Variables|Default|GetActionNameForB))
        (Timeline|TL_MoveDoor Reverse)))))

(fn ConstructionScript
  (|CallParentFunction))